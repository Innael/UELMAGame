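; Game mode for the second level that runs music, a countdown and enemy-fall progression.
; On start it sets the level in the game instance and copies its saved score to the player.
; A looping one-second timer counts down, then pauses the game and shows the time-off menu with the score.
; Enemy falls reaching a threshold fire the first-dialog dispatcher, which stops the music, then a second threshold fires the end dispatcher.
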(event Custom|EnemyFallPlus
  (if (Variables|Default|GetFL_FirstDialogCheck)
    (Variables|Default|SetEnemyFallsCount (+ (Variables|Default|GetEnemyFallsCount) 1))
    (if (>= (Variables|Default|GetEnemyFallsCount) (Variables|Default|GetEnemyFallsCheck))
      (Default|CallFLEndDispatcher))
    (else
      (Variables|Default|SetEnemyFallsCount (+ (Variables|Default|GetEnemyFallsCount) 1))
      (if (>= (Variables|Default|GetEnemyFallsCount) (Variables|Default|GetEnemyFallsCheck))
        (Variables|Default|SetEnemyFallsCount 0)
        (Variables|Default|SetEnemyFallsCheck 100)
        (Default|CallFLFirsDialogDispatcher)
        (Variables|Default|SetFL_FirstDialogCheck true)))))

(event Custom|CustomEvent
  (bind _returnvalue (Game|GetPlayerController 0))
  (bind _output_get (Variables|Default|SetGame%20Time (- (Variables|Default|GetGame%20Time) 1)))
  (if (== _output_get 0)
    (Utilities|Time|ClearandInvalidateTimerbyHandle (Variables|Default|GetGameTimerHandle))
    (Game|SetGamePaused true)
    (bind _returnvalue_2 (UserInterface|CreateWidget "/Game/LeaveMeAlone/Widgets/UI/WBP_TimeOff_Menu.WBP_TimeOff_Menu_C"))
    (bind _output_get_2 (Variables|Default|SetTimeOffWidget _returnvalue_2))
    (UserInterface|Viewport|AddtoViewport _output_get_2 0)
    (Utilities|FlowControl|Sequence
      (:then_0
        (Input|SetInputModeUIOnly _returnvalue 0 "DoNotLock" false)
        (Variables|/Script/Engine.PlayerController|SetbShowMouseCursor _returnvalue true))
      (:then_1
        (bind _asch_player (Utilities|Casting|CastToCH_Player (Game|GetPlayerCharacter 0)))
        (Variables|/Game/LeaveMeAlone/Widgets/UI/WBP_TimeOff_Menu.WBP_TimeOff_Menu_C|SetTimeScore _returnvalue_2 (Variables|/Game/LeaveMeAlone/Core/Characters/CH_Player.CH_Player_C|GetScore _asch_player))))))

(event Custom|Stop%20Music
  (Utilities|FlowControl|Delay 4.5)
  (Audio|Components|Audio|Stop (Variables|Default|GetLevelMusic)))

(event EventBeginPlay
  (bind _levelmusic (Variables|Default|GetLevelMusic))
  (Utilities|FlowControl|Sequence
    (:then_0
      (Audio|Components|Audio|SetSound _levelmusic "/Game/RPG_Music_Lite_II/WAVs/War_of_Exploding_Mountains/Loops/War_of_Exploding_Mountains_V1_Loop.War_of_Exploding_Mountains_V1_Loop")
      (Audio|Components|Audio|Play _levelmusic 0.0)
      (EventDispatchers|BindEventtoFLFirsDialogDispatcher (delegate Custom|Stop%20Music)))
    (:then_1
      (bind _returnvalue (Utilities|Time|SetTimerbyEvent (delegate Custom|CustomEvent) 1.0 true))
      (Variables|Default|SetGameTimerHandle _returnvalue))
    (:then_2
      (EventDispatchers|BindEventtoEnemyFallDispatcher (delegate Custom|EnemyFallPlus)))
    (:then_3
      (bind _asgi_leave_me_alone (Utilities|Casting|CastToGI_LeaveMeAlone (Game|GetGameInstance)))
      (Variables|/Game/LeaveMeAlone/Core/GameInstance/GI_LeaveMeAlone.GI_LeaveMeAlone_C|SetLevel _asgi_leave_me_alone 2)
      (bind _asch_player (Utilities|Casting|CastToCH_Player (Game|GetPlayerCharacter 0)))
      (Variables|/Game/LeaveMeAlone/Core/Characters/CH_Player.CH_Player_C|SetScore _asch_player (Variables|/Game/LeaveMeAlone/Core/GameInstance/GI_LeaveMeAlone.GI_LeaveMeAlone_C|GetScore _asgi_leave_me_alone)))))

(event EventTick
  (params (DeltaSeconds :type Float%20%28single-precision%29)))

(fn ConstructionScript)