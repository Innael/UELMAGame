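; Game mode for LeaveMeAlone that runs the match countdown and ends play when time runs out.
; BeginPlay starts looping music after a short delay and a repeating one-second timer that decrements GameTime.
; At zero it clears the timer, pauses the game, shows the time-off menu widget and switches to UI-only input with a visible cursor.
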(event Custom|CustomEvent
  (bind _returnvalue (Game|GetPlayerController 0))
  (bind _output_get (Variables|Default|SetGame%20Time (- (Variables|Default|GetGame%20Time) 1)))
  (if (== _output_get 0)
    (Utilities|Time|ClearandInvalidateTimerbyHandle (Variables|Default|GetGameTimerHandle))
    (Game|SetGamePaused true)
    (bind _returnvalue_2 (UserInterface|CreateWidget "/Game/LeaveMeAlone/Widgets/UI/WPB_TimeOff_Menu.WPB_TimeOff_Menu_C"))
    (bind _output_get_2 (Variables|Default|SetTimeOffWidget _returnvalue_2))
    (UserInterface|Viewport|AddtoViewport _output_get_2 0)
    (Input|SetInputModeUIOnly _returnvalue _returnvalue_2 "DoNotLock" false)
    (Variables|/Script/Engine.PlayerController|SetbShowMouseCursor _returnvalue true)))

(event EventBeginPlay
  (Utilities|FlowControl|Sequence
    (:then_0
      (Utilities|FlowControl|Delay 5.0)
      (Audio|PlaySound2D "/Game/RPG_Music_Lite_II/WAVs/War_of_Exploding_Mountains/Loops/War_of_Exploding_Mountains_V1_Loop.War_of_Exploding_Mountains_V1_Loop" 0.5 1.0 0.0 0 0))
    (:then_1
      (bind _returnvalue (Utilities|Time|SetTimerbyEvent (delegate Custom|CustomEvent) 1.0 true))
      (Variables|Default|SetGameTimerHandle _returnvalue))))

(event EventTick
  (params (DeltaSeconds :type Float%20%28single-precision%29)))

(fn ConstructionScript)